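; Exit door actor that serves as the extraction point where the player delivers carried gnomes to win.
; When the first-person character overlaps its box while holding a gnome, it clears the held state, hides the gnome mesh and plays a sound.
; It increments the character's exfiled gnome count, then calls the character's Win once the needed total is reached, otherwise prints the count.
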(event OnComponentBeginOverlap(Box)
  (params (OverlappedComponent :type Primitive%20Component%20Object%20Reference) (OtherActor :type Actor%20Object%20Reference) (OtherComp :type Primitive%20Component%20Object%20Reference) (OtherBodyIndex :type Integer) (bFromSweep :type Boolean) (SweepResult :type Hit%20Result%20Structure%20%28by%20ref%29))
  (bind _asbp_first_person_character (Utilities|Casting|CastToBP_FirstPersonCharacter OtherActor))
  (if (Variables|/Game/FirstPerson/Blueprints/BP_FirstPersonCharacter.BP_FirstPersonCharacter_C|GetIsGnomeBeingHeld? _asbp_first_person_character)
    (Variables|/Game/FirstPerson/Blueprints/BP_FirstPersonCharacter.BP_FirstPersonCharacter_C|SetIsGnomeBeingHeld? _asbp_first_person_character false)
    (Rendering|SetVisibility (Variables|/Game/FirstPerson/Blueprints/BP_FirstPersonCharacter.BP_FirstPersonCharacter_C|GetGnomeMesh _asbp_first_person_character) false false)
    (Audio|PlaySound2D "/Game/MyStuff/Audio/Go_Again.Go_Again" 1.0 1.0 0.0 0 0)
    (bind _result (Math|Integer|IncrementInt (Variables|/Game/FirstPerson/Blueprints/BP_FirstPersonCharacter.BP_FirstPersonCharacter_C|GetExfiled%20Gnomes _asbp_first_person_character))
      (:%20%20
        (bind _output_get (Variables|/Game/FirstPerson/Blueprints/BP_FirstPersonCharacter.BP_FirstPersonCharacter_C|SetExfiled%20Gnomes _asbp_first_person_character _result))
        (if (>= _output_get (Variables|/Game/FirstPerson/Blueprints/BP_FirstPersonCharacter.BP_FirstPersonCharacter_C|GetGnomes%20Needed _asbp_first_person_character))
          (Default|Win _asbp_first_person_character)
          (else
            (Development|PrintString (Utilities|String|ToString(Integer) _output_get))))))))

(event EventBeginPlay)

(event Collision|EventActorBeginOverlap
  (params (OtherActor :type Actor%20Object%20Reference)))

(event EventTick
  (params (DeltaSeconds :type Float%20%28single-precision%29)))

(fn ConstructionScript)