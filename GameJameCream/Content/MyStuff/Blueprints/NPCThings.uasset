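; An NPC character Blueprint that gives each instance a random skin and sends it wandering the level.
; On BeginPlay it sets a random material from CharacterSkinArray, then moves via AIMoveTo to random navigable points around its current location, repeating after each successful move.
; Tick disables character movement while the Alerted flag is set.
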(event EventBeginPlay
  (Rendering|Material|SetMaterial (Variables|Character|GetMesh) 0 (Utilities|Array|Get(acopy) (Variables|Default|GetCharacterSkinArray) (Math|Random|RandomIntegerinRange 0 7)))
  (bind _randomlocation (Class|NavigationSystemV1|GetRandomLocationinNavigableRadius (Transformation|GetActorLocation) 5e+02 0 0 :!label _label))
  (AI|AIMoveTo self _randomlocation 0 5.0 false
    (:OnSuccess
      (goto _label))))

(event Collision|EventActorBeginOverlap
  (params (OtherActor :type Actor%20Object%20Reference)))

(event EventTick
  (params (DeltaSeconds :type Float%20%28single-precision%29))
  (if (Variables|Default|GetAlerted)
    (Pawn|Components|CharacterMovement|DisableMovement (Variables|Character|GetCharacterMovement))))

(fn ConstructionScript)