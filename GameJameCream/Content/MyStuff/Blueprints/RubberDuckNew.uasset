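; Rubber duck AI pawn that hunts the first-person player once the player's alert total reaches the death threshold.
; Tick polls that count, then sets Enabled and calls Attack every frame while the threshold holds.
; Attack issues an AI MoveTo on the player, re-issued on success, and plays a Quack at the duck's capsule, throttled by a DoOnce that resets after a short delay.
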(event Custom|Attack
  (bind _asbp_first_person_character (Utilities|Casting|CastToBP_FirstPersonCharacter (Game|GetPlayerCharacter 0) :!label _label))
  (AI|AIMoveTo self "0, 0, 0" _asbp_first_person_character 5.0 false
    (:then
      (Utilities|FlowControl|DoOnce false :!label _label_2
        (:Completed
          (Audio|PlaySoundatLocation "/Game/MyStuff/Audio/quack.quack" (Transformation|GetWorldLocation (Variables|Collision|GetCapsuleComponent)) "0, 0, 0" 1.0 1.0 0.0 0 0 0 0)
          (Utilities|FlowControl|Delay 0.3)
          (goto _label_2 Reset))))
    (:OnSuccess
      (goto _label))))

(event EventTick
  (params (DeltaSeconds :type Float%20%28single-precision%29))
  (bind _asbp_first_person_character (Utilities|Casting|CastToBP_FirstPersonCharacter (Game|GetPlayerCharacter 0)))
  (if (>= (Variables|/Game/FirstPerson/Blueprints/BP_FirstPersonCharacter.BP_FirstPersonCharacter_C|GetTotal%20Alerted _asbp_first_person_character) (Variables|/Game/FirstPerson/Blueprints/BP_FirstPersonCharacter.BP_FirstPersonCharacter_C|GetTotalALertsBeforeDeath _asbp_first_person_character))
    (Variables|Default|SetEnabled true)
    (CallFunction|Attack)))

(fn ConstructionScript)