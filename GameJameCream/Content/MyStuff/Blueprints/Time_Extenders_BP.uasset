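; Time extender actor that adds TimeToAdd to the first-person character's TimerValue when interacted with.
; A Sphere overlap swaps ExtenderMesh to the Trippy material and shows the character's interact widget, and end overlap sets BAeballBat and removes the widget.
; The Interact event acts on player 0's character and neither checks overlap nor consumes the extender.
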(event OnComponentBeginOverlap(Sphere)
  (params (OverlappedComponent :type Primitive%20Component%20Object%20Reference) (OtherActor :type Actor%20Object%20Reference) (OtherComp :type Primitive%20Component%20Object%20Reference) (OtherBodyIndex :type Integer) (bFromSweep :type Boolean) (SweepResult :type Hit%20Result%20Structure%20%28by%20ref%29))
  (bind _asbp_first_person_character (Utilities|Casting|CastToBP_FirstPersonCharacter OtherActor))
  (Rendering|Material|SetMaterial (Variables|Default|GetExtenderMesh) 0 "/Game/MyStuff/Materials/Trippy.Trippy")
  (Default|AddInteractWidget _asbp_first_person_character))

(event OnComponentEndOverlap(Sphere)
  (params (OverlappedComponent :type Primitive%20Component%20Object%20Reference) (OtherActor :type Actor%20Object%20Reference) (OtherComp :type Primitive%20Component%20Object%20Reference) (OtherBodyIndex :type Integer))
  (bind _asbp_first_person_character (Utilities|Casting|CastToBP_FirstPersonCharacter OtherActor))
  (Rendering|Material|SetMaterial (Variables|Default|GetExtenderMesh) 0 "/Game/MyStuff/Materials/Baseball_Bat/BAeballBat.BAeballBat")
  (Default|RemoveInteractWidget _asbp_first_person_character))

(event EventBeginPlay)

(event EventTick
  (params (DeltaSeconds :type Float%20%28single-precision%29)))

(event EventInteract
  (bind _asbp_first_person_character (Utilities|Casting|CastToBP_FirstPersonCharacter (Game|GetPlayerCharacter 0)))
  (Variables|/Game/FirstPerson/Blueprints/BP_FirstPersonCharacter.BP_FirstPersonCharacter_C|SetTimer%20Value _asbp_first_person_character (+ (Variables|/Game/FirstPerson/Blueprints/BP_FirstPersonCharacter.BP_FirstPersonCharacter_C|GetTimer%20Value _asbp_first_person_character) (Variables|Default|GetTime%20to%20add))))

(fn ConstructionScript)